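; Zone Blueprint that picks which of its Food, Wealth or Technology stats to report as a subject name, possibly dishonestly.
; GetRndSubject names the lowest stat when truthful and the highest when lying, mapping the value back to a name through ChooseSubject.
; IsLying rolls against Control: a coin flip when low, a small fixed chance when high, otherwise likelier lies as Control drops.
; Decay and the construction script are empty, and debug prints remain.
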(fn `ChooseSubject`
  (params (Field :type "Float (double-precision)"))
  (returns (Subject :type String))
  (locals (SubjectName :type String))
  (if (== Field (`self.Food`))
    (set `local.SubjectName` "Food")
    (return (`local.SubjectName`))
    (elif (== Field (`self.Wealth`))
      (set `local.SubjectName` "Economy")
      (return (`local.SubjectName`))
      (elif (== Field (`self.Technology`))
        (set `local.SubjectName` "Technology")
        (return (`local.SubjectName`))))))

(fn `Decay`)

(fn `GetRndSubject`
  (returns (Subject :type String))
  (locals (Lying :type Boolean) (SubjectName :type String :default "Food") (ChosenField :type "Float (double-precision)"))
  (bind _subjectname (`local.SubjectName`))
  (bind _lying (`self.IsLying`))
  (bind _output_get (set `local.Lying` _lying))
  (`KismetSystemLibrary.PrintString` (`KismetStringLibrary.Conv_BoolToString` _output_get))
  (if _output_get
    (bind _output_get_2 (set `local.ChosenField` (`KismetMathLibrary.FMax` (`self.Food`) (`self.Wealth`) (`self.Technology`))))
    (bind _subject (`self.ChooseSubject` _output_get_2))
    (set `local.SubjectName` _subject)
    (else
      (bind _output_get_3 (set `local.ChosenField` (`KismetMathLibrary.FMin` (`self.Food`) (`self.Wealth`) (`self.Technology`))))
      (bind _subject_2 (`self.ChooseSubject` _output_get_3))
      (set `local.SubjectName` _subject_2)))
  (`KismetSystemLibrary.PrintString` _subjectname true true (struct :`G` 1.0 :`B` 0.307963 :`A` 1.0))
  (return _subjectname))

(fn `IsLying`
  (returns (Lying :type Boolean))
  (locals (Is_Lying :type Boolean))
  (if (<= (`self.Control`) 20.0)
    (set `local.Is_Lying` (`KismetMathLibrary.RandomBool`))
    (elif (>= (`self.Control`) 80.0)
      (set `local.Is_Lying` (<= (`KismetMathLibrary.RandomInteger` 10) 1))
      (else
        (set `local.Is_Lying` (>= (`KismetMathLibrary.RandomFloatInRange` 0.0 (`self.JaugeMax`)) (`self.Control`))))))
  (return (`local.Is_Lying`)))

(fn `UserConstructionScript`)