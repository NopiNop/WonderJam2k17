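; Base paper-sprite NPC that wanders a zone, turning at walls, with randomized Food, Wealth and Technology needs that decay over time.
; A mouse click or a need reaching the threshold sends it into Zone2's waiting-room queue, where the HUD may spawn the next one.
; Entering a trigger box halts it to ask.
; Its request names its lowest need, or its highest when lying, decided randomly from Dissidence.
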(event `self.ReceiveBeginPlay`
  (bind _capsulecomponent (`self.CapsuleComponent`))
  (if (not (`self.inWaitingRoom`))
    (`PrimitiveComponent.SetCollisionResponseToChannel` _capsulecomponent "ECC_WorldDynamic" "ECR_Ignore")
    (`PrimitiveComponent.SetCollisionResponseToChannel` _capsulecomponent "ECC_PhysicsBody" "ECR_Ignore")
    (`PrimitiveComponent.SetCollisionResponseToChannel` _capsulecomponent "ECC_Pawn" "ECR_Ignore")))

(event `self.ReceiveActorBeginOverlap`
  (params (OtherActor :type "Actor Object Reference"))
  (cast `TriggerBox` OtherActor)
  (set `self.MovementDirection` (0.0 0.0 0.0))
  (set `self.IsAsking` true))

(event `self.ReceiveHit`
  (params (MyComp :type "PrimitiveComponent Object Reference") (Other :type "Actor Object Reference") (OtherComp :type "PrimitiveComponent Object Reference") (bSelfMoved :type Boolean) (HitLocation :type "Vector Structure") (HitNormal :type "Vector Structure") (NormalImpulse :type "Vector Structure") (Hit :type "HitResult Structure (by ref)"))
  (if (`KismetStringLibrary.Contains` (`KismetSystemLibrary.GetDisplayName` Other) "Wall")
    (bind _result (`/Engine/EditorBlueprintResources/StandardMacros.NegateFloat` (.x (`self.MovementDirection`)))
      (:`  `
        (set `self.MovementDirection` (`KismetMathLibrary.MakeVector` _result (.y (`self.MovementDirection`)) (.z (`self.MovementDirection`))))))))

(event `self.ReceiveTick`
  (params (DeltaSeconds :type "Float (single-precision)"))
  (bind _movementdirection_x (`KismetMathLibrary.BreakVector` (`self.MovementDirection`)))
  (if (not (`self.inWaitingRoom`))
    (`self.DecayOverTime` DeltaSeconds)
    (`self.CheckRessources`))
  (`self.AddMovementInput` (`self.MovementDirection`) (`self.MovementSpeed`))
  (if (`self.inWaitingRoom`)
    _
    (elif (<= _movementdirection_x 0.0)
      (`self.K2_SetActorRotation` (struct :`Yaw` 180.0))
      (else
        (`self.K2_SetActorRotation` (struct))))))

(event `Key|LeftMouseButton`
  (params (Key :type "Key Structure" :default "AnyKey"))
  ;[1 1 1] on clicked actor add to waiting room
  (:`Pressed`
    (bind _asbase_npc (cast `/Game/Blueprints/BaseNPC` (`.HitActor` (`GameplayStatics.BreakHitResult` (`PlayerController.GetHitResultUnderCursorByChannel` (`GameplayStatics.GetPlayerController` 0) "TraceTypeQuery1" true)))))
    (if (not (`/Game/Blueprints/BaseNPC.inWaitingRoom` _asbase_npc))
      (`SceneComponent.SetVisibility` (`/Game/Blueprints/BaseNPC.convokedText` _asbase_npc) true true)
      (`self.GoToWaitingRoom` _asbase_npc))))

(fn `CheckRessources`
  (locals (Seuil :type "Float (double-precision)" :default 30.0))
  (if (or (<= (`self.Food`) (`local.Seuil`)) (<= (`self.Technology`) (`local.Seuil`)) (<= (`self.Wealth`) (`local.Seuil`)))
    (`self.GoToWaitingRoom`)))

(fn `ChooseSubject`
  (params (Field :type "Float (double-precision)"))
  (returns (Subject :type String))
  (locals (SubjectName :type String))
  (if (== Field (`self.Food`))
    (set `local.SubjectName` "Food")
    (return (`local.SubjectName`))
    (elif (== Field (`self.Wealth`))
      (set `local.SubjectName` "Economy")
      (return (`local.SubjectName`))
      (elif (== Field (`self.Technology`))
        (set `local.SubjectName` "Technology")
        (return (`local.SubjectName`))))))

(fn `DecayOverTime`
  (params (DeltaTime :type "Float (double-precision)"))
  (bind _output_get (set `self.Time` (+ DeltaTime (`self.Time`))))
  (if (>= _output_get 2.0)
    (set `self.Time` 0.0)
    (set `self.Food` (- (`self.Food`) (`self.FoodDecay`)))
    (set `self.Technology` (- (`self.Technology`) (`self.TechnoDecay`)))
    (set `self.Wealth` (- (`self.Wealth`) (`self.WealthDecay`)))))

(fn `DetectDissidence`
  (if (>= (`self.Dissidence`) 50.0)
    (`PaperFlipbookComponent.SetFlipbook` (`self.Sprite`) null)))

(fn `DisableActor`
  (bind _capsulecomponent (`self.CapsuleComponent`))
  (`PrimitiveComponent.SetCollisionResponseToChannel` _capsulecomponent "ECC_WorldDynamic" "ECR_Ignore")
  (`PrimitiveComponent.SetCollisionResponseToChannel` _capsulecomponent "ECC_PhysicsBody" "ECR_Ignore")
  (`PrimitiveComponent.SetCollisionResponseToChannel` _capsulecomponent "ECC_Pawn" "ECR_Ignore")
  (set `self.MovementDirection` (0.0 0.0 0.0))
  (set `CharacterMovementComponent.GravityScale` 0.0 (`self.CharacterMovement`))
  (set `self.MovementSpeed` 0.0)
  (`ActorComponent.SetComponentTickEnabled` (`self.CharacterMovement`) false))

(fn `EnableActor`
  (bind _capsulecomponent (`self.CapsuleComponent`))
  (set `CharacterMovementComponent.GravityScale` 1.0 (`self.CharacterMovement`))
  (set `self.MovementSpeed` 0.4)
  (`self.K2_SetActorRotation` (struct))
  (`self.SetActorScale3D` (1.0 1.0 1.0))
  (set `self.MovementDirection` (1.0 0.0 0.0))
  (`ActorComponent.SetComponentTickEnabled` (`self.CharacterMovement`) true)
  (`PrimitiveComponent.SetCollisionResponseToChannel` _capsulecomponent "ECC_WorldDynamic" "ECR_Ignore")
  (`PrimitiveComponent.SetCollisionResponseToChannel` _capsulecomponent "ECC_PhysicsBody" "ECR_Block")
  (`PrimitiveComponent.SetCollisionResponseToChannel` _capsulecomponent "ECC_Pawn" "ECR_Block"))

(fn `GetBackToZone`
  (params (Location :type "Vector Structure"))
  (bind _capsulecomponent (`self.CapsuleComponent`))
  (`self.SetActorScale3D` (0.3 0.3 0.3))
  (set `self.MovementDirection` (1.0 0.0 0.0))
  (set `self.inWaitingRoom` false)
  (`self.K2_TeleportTo` Location (struct))
  (`PrimitiveComponent.SetCollisionResponseToChannel` _capsulecomponent "ECC_WorldDynamic" "ECR_Ignore")
  (`PrimitiveComponent.SetCollisionResponseToChannel` _capsulecomponent "ECC_PhysicsBody" "ECR_Ignore")
  (`PrimitiveComponent.SetCollisionResponseToChannel` _capsulecomponent "ECC_Pawn" "ECR_Ignore"))

(fn `GetRndSubject`
  (returns (Subject :type String))
  (locals (SubjectName :type String) (Lying :type Boolean) (ChosenField :type "Float (double-precision)"))
  (bind _lying (`self.IsLying`))
  (bind _output_get (set `local.Lying` _lying))
  (if _output_get
    (bind _output_get_2 (set `local.ChosenField` (`KismetMathLibrary.FMax` (`self.Food`) (`self.Wealth`) (`self.Technology`))))
    (bind _subject (`self.ChooseSubject` _output_get_2))
    (set `local.SubjectName` _subject)
    (else
      (bind _output_get_3 (set `local.ChosenField` (`KismetMathLibrary.FMin` (`self.Food`) (`self.Wealth`) (`self.Technology`))))
      (bind _subject_2 (`self.ChooseSubject` _output_get_3))
      (set `local.SubjectName` _subject_2)))
  (return (`local.SubjectName`)))

(fn `GoToWaitingRoom`
  (locals (Zone2 :type "/Game/Blueprints/Zone Object Reference"))
  (set `self.inWaitingRoom` true)
  (`self.DisableActor`)
  (bind _outactors (`GameplayStatics.GetAllActorsOfClass` "/Game/Blueprints/Zone.Zone_C"))
  (for _array_element _outactors
    (set `local.Zone2` _array_element)
    (if (`KismetStringLibrary.EqualEqual_StrStr` (`KismetSystemLibrary.GetDisplayName` _array_element) "Zone2")
      (`KismetArrayLibrary.Array_Add` (`/Game/Blueprints/Zone.Queue` (`local.Zone2`)) self)
      (bind _outactors_2 (`GameplayStatics.GetAllActorsOfClass` "/Script/Engine.TargetPoint"))
      (for _array_element_2 _outactors_2
        (if (`KismetStringLibrary.EqualEqual_StrStr` (`KismetSystemLibrary.GetDisplayName` _array_element_2) "TargetPoint")
          (`self.K2_TeleportTo` (`self.K2_GetActorLocation` _array_element_2))
          (`KismetSystemLibrary.PrintString` "Hello")
          (if (<= (`KismetArrayLibrary.Array_Length` (`/Game/Blueprints/Zone.Queue` (`local.Zone2`))) 3)
            (bind _foundwidgets (`WidgetBlueprintLibrary.GetAllWidgetsOfClass` "/Game/HUD.HUD_C"))
            (`/Game/HUD.SpawnNext` (`KismetArrayLibrary.Array_Get` _foundwidgets))))))))

(fn `IsLying`
  (returns (Lying :type Boolean))
  (locals (Is_Lying :type Boolean))
  (if (<= (`self.Dissidence`) 20.0)
    (set `local.Is_Lying` (`KismetMathLibrary.RandomBool`))
    (elif (>= (`self.Dissidence`) 80.0)
      (set `local.Is_Lying` (<= (`KismetMathLibrary.RandomInteger` 10) 1))
      (else
        (set `local.Is_Lying` (>= (`KismetMathLibrary.RandomFloatInRange` 0.0 100.0) (`self.Dissidence`))))))
  (return (`local.Is_Lying`)))

(fn `ResetFood`
  (set `self.Food` (`self.RessourceMax`)))

(fn `ResetTechno`
  (set `self.Technology` (`self.RessourceMax`)))

(fn `ResetWealth`
  (set `self.Wealth` (`self.RessourceMax`)))

(fn `UserConstructionScript`
  (bind _returnvalue (`KismetMathLibrary.RandomFloatInRange` 50.0 100.0))
  (bind _capsulecomponent (`self.CapsuleComponent`))
  (set `self.Wealth` _returnvalue)
  (set `self.Technology` _returnvalue)
  (set `self.Food` _returnvalue)
  (if (`self.inWaitingRoom`)
    (`SceneComponent.SetRelativeScale3D` _capsulecomponent (1.0 1.0 1.0))
    (else
      (`SceneComponent.SetRelativeScale3D` _capsulecomponent (0.3 0.3 0.3))
      (set `CharacterMovementComponent.MaxWalkSpeed` 200.0 (`self.CharacterMovement`)))))