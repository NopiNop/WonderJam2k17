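; RichNPC is a rich civilian NPC Blueprint that changes its walk animation to show rebellion.
; It overrides little event logic, leaving Tick and construction to its parent class.
; DetectDissidence switches the sprite to the rebel rich walk flipbook once Dissidence reaches a threshold, and UndetectDissidence restores the normal rich walk.
; Both functions always return false.
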(event `self.ReceiveTick`
  (params (DeltaSeconds :type "Float (single-precision)"))
  (`parent.ReceiveTick` DeltaSeconds))

(fn `DetectDissidence`
  (returns (return :type Boolean))
  (if (>= (`self.Dissidence`) 50.0)
    (`PaperFlipbookComponent.SetFlipbook` (`self.Sprite`) "/Game/Sprites/Character/animations/Rich/Flip_RebelRichWalk.Flip_RebelRichWalk"))
  (return false))

(fn `UndetectDissidence`
  (returns (return :type Boolean))
  (`PaperFlipbookComponent.SetFlipbook` (`self.Sprite`) "/Game/Sprites/Character/animations/Rich/Flip_RichWalk.Flip_RichWalk")
  (return false))

(fn `UserConstructionScript`
  (`parent.UserConstructionScript`))