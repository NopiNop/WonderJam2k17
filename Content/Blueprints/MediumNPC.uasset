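; MediumNPC is a Paper2D NPC Blueprint that switches its visual depending on whether it is in a waiting room.
; Each Tick runs the parent logic, then checks InWaitingRoom to show either the static PaperSprite or the animated Sprite flipbook component.
; Outside the waiting room, the flipbook component plays the Flip_MiddleWalk walk animation.
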(event `self.ReceiveTick`
  (params (DeltaSeconds :type "Float (single-precision)"))
  (bind _papersprite (`self.PaperSprite`))
  (bind _sprite (`self.Sprite`))
  (`parent.ReceiveTick` DeltaSeconds)
  ;[1 1 1] Walk animation
  (if (`self.inWaitingRoom`)
    (`SceneComponent.SetVisibility` _papersprite true false)
    (`SceneComponent.SetVisibility` _sprite false false)
    (else
      (`SceneComponent.SetVisibility` _papersprite false false)
      (`SceneComponent.SetVisibility` _sprite true false)
      (`PaperFlipbookComponent.SetFlipbook` _sprite "/Game/Sprites/Character/animations/Middle/Flip_MiddleWalk.Flip_MiddleWalk"))))

(fn `UserConstructionScript`
  (`parent.UserConstructionScript`))