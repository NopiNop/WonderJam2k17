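; PoorNPC is an NPC Blueprint whose Paper2D flipbook sprite can reveal whether it is a rebel.
; DetectDissidence switches the sprite to the rebel walk flipbook when Dissidence reaches a threshold, and UndetectDissidence restores the normal poor walk.
; Both functions always return false; Tick and construction only call the parent, and the overlap event is disabled.
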(event `self.ReceiveTick`
  (params (DeltaSeconds :type "Float (single-precision)"))
  (`parent.ReceiveTick` DeltaSeconds))

(fn `DetectDissidence`
  (returns (return :type Boolean))
  (if (>= (`self.Dissidence`) 50.0)
    (`PaperFlipbookComponent.SetFlipbook` (`self.Sprite`) "/Game/Sprites/Character/animations/Poor/Flip_RebelPoorWalk.Flip_RebelPoorWalk"))
  (return false))

(fn `UndetectDissidence`
  (returns (return :type Boolean))
  (`PaperFlipbookComponent.SetFlipbook` (`self.Sprite`) "/Game/Sprites/Character/animations/Poor/Flip_PoorWalk.Flip_PoorWalk")
  (return false))

(fn `UserConstructionScript`
  (`parent.UserConstructionScript`))